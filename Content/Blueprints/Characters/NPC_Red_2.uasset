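; Red-team NPC for an auto-battle that chases and fights NPC_Blue_2 characters.
; BeginPlay moves it toward the nearest living Blue; Tick keeps it jumping and, after a delay, retargets upon finding dead Blues, printing "RED WINS" when all are counted dead.
; Hits from Blues deal random damage and knockback; at zero health it ragdolls and swaps its parent child-actor class to plain Actor.
; Dead bodies disable collision on Blue overlap.
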(event `self.ReceiveBeginPlay`
  (bind _outactors (`GameplayStatics.GetAllActorsOfClass` "/Game/Blueprints/Characters/NPC_Blue_2.NPC_Blue_2_C" :!label _label))
  (for _array_element _outactors
    (if (not (`/Game/Blueprints/Characters/NPC_Blue_2.isDead` _array_element))
      (bind _returnvalue (`self.GetDistanceTo` _array_element))
      (`/Engine/EditorBlueprintResources/StandardMacros.CompareFloat` _returnvalue (`self.LowerDistance`)
        (:`<`
          (set `self.LowerDistance` _returnvalue)
          (bind _output_get (set `self.CurrentTarget` _array_element))
          (`NavigationSystem.SimpleMoveToActor` (`self.GetController`) _output_get :!label _label_2)))))
  (goto _label_2))

(event `self.ReceiveTick`
  (params (DeltaSeconds :type "Float (single-precision)"))
  (if (`self.isDead`)
    (`CharacterMovementComponent.DisableMovement` (`self.CharacterMovement`))
    (`self.StopJumping`)
    (else
      (`self.Jump`)
      (`KismetSystemLibrary.Delay` 1.0)
      (bind _outactors (`GameplayStatics.GetAllActorsOfClass` "/Game/Blueprints/Characters/NPC_Blue_2.NPC_Blue_2_C"))
      (for _array_element _outactors
        (if (`/Game/Blueprints/Characters/NPC_Blue_2.isDead` _array_element)
          (set `self.DeadEnemyCount` (+ (`self.DeadEnemyCount`) 1))
          (goto _label)))
      (if (< (`self.DeadEnemyCount`) (`KismetArrayLibrary.Array_Length` _outactors))
        (set `self.DeadEnemyCount` 0)
        (else
          (`KismetSystemLibrary.PrintString` "RED WINS" true true (struct :`R` 1.0 :`B` 0.011234 :`A` 1.0) 1.0))))))

(event `self.ReceiveActorBeginOverlap`
  (params (OtherActor :type "Actor Object Reference")))

(event `self.ReceiveHit`
  (params (MyComp :type "PrimitiveComponent Object Reference") (Other :type "Actor Object Reference") (OtherComp :type "PrimitiveComponent Object Reference") (bSelfMoved :type Boolean) (HitLocation :type "Vector Structure") (HitNormal :type "Vector Structure") (NormalImpulse :type "Vector Structure") (Hit :type "HitResult Structure (by ref)"))
  (bind _mesh (`self.Mesh`))
  (if (`self.isDead`)
    _
    (elif (== (`GameplayStatics.GetObjectClass` Other) "/Game/Blueprints/Characters/NPC_Blue_2.NPC_Blue_2_C")
      (bind _output_get (set `self.Health` (- (`self.Health`) (`KismetMathLibrary.RandomFloatInRange` 10.0 15.0))))
      (`self.LaunchCharacter` (* (`self.GetActorForwardVector` Other) 200.0))
      (if (<= _output_get 0.0)
        (`PrimitiveComponent.SetSimulatePhysics` _mesh true)
        (`PrimitiveComponent.SetSimulatePhysics` (`self.CapsuleComponent`) true)
        (`PrimitiveComponent.SetCollisionEnabled` _mesh "PhysicsOnly")
        (set `self.isDead` true)
        (`self.StopJumping`)
        (`ChildActorComponent.SetChildActorClass` (`self.GetParentComponent`) "/Script/Engine.Actor")))))

(event `self.CapsuleComponent.OnComponentBeginOverlap`
  (params (OverlappedComponent :type "PrimitiveComponent Object Reference") (OtherActor :type "Actor Object Reference") (OtherComp :type "PrimitiveComponent Object Reference") (OtherBodyIndex :type Integer) (bFromSweep :type Boolean) (SweepResult :type "HitResult Structure (by ref)"))
  (if (`self.isDead`)
    (if (== (`GameplayStatics.GetObjectClass` OtherActor) "/Game/Blueprints/Characters/NPC_Blue_2.NPC_Blue_2_C")
      (`PrimitiveComponent.SetCollisionEnabled` OverlappedComponent "NoCollision"))))

(event `self.Mesh.OnComponentBeginOverlap`
  (params (OverlappedComponent :type "PrimitiveComponent Object Reference") (OtherActor :type "Actor Object Reference") (OtherComp :type "PrimitiveComponent Object Reference") (OtherBodyIndex :type Integer) (bFromSweep :type Boolean) (SweepResult :type "HitResult Structure (by ref)"))
  (if (`self.isDead`)
    (if (== (`GameplayStatics.GetObjectClass` OtherActor) "/Game/Blueprints/Characters/NPC_Blue_2.NPC_Blue_2_C")
      (`PrimitiveComponent.SetCollisionEnabled` OverlappedComponent "NoCollision"))))

(fn `UserConstructionScript`)