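; Team B NPC character that automatically battles NPC_TeamA, hopping while alive and ragdolling at zero health.
; Tick, throttled by a random Delay, picks the nearest living enemy and chases it, returning to spawn when none remain; capsule hits also retarget.
; On overlap, a random "Janken" roll beating the target's deals damage, launch and explosion, rerolling ties.
; A screen-projected UI_Stats widget shows NPC and target status while the player overlaps its Sphere.
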(event `self.ReceiveBeginPlay`
  (`self.CreateWidget`)
  (`SceneComponent.K2_AttachToComponent` (`self.Sphere`) (`self.Mesh`) "None" "SnapToTarget" "KeepRelative" "KeepRelative" true)
  (set `self.SpawnLocation` (`self.K2_GetActorLocation`))
  (set `self.Janken` (`KismetMathLibrary.RandomIntegerInRange` 0 100)))

(event `self.ReceiveTick`
  (params (DeltaSeconds :type "Float (single-precision)"))
  (bind _returnvalue (`KismetMathLibrary.RandomFloatInRange` 1.0 5.0))
  (bind _returnvalue_2 (`KismetMathLibrary.RandomFloatInRange` 300.0 500.0))
  (bind _currenttarget (`self.CurrentTarget`))
  (bind _enemyfindingrange (`self.EnemyFindingRange`))
  (bind _ui_stats (`self.UI Stats`))
  (bind _ui_stats_2 (`self.UI Stats`))
  (bind _currenttarget_2 (`self.CurrentTarget`))
  (bind _mesh (`self.Mesh`))
  (bind _janken (`/Game/Blueprints/Characters/NPC_TeamA.Janken` (`self.CurrentTarget`)))
  (if (`PrimitiveComponent.IsOverlappingActor` (`self.Sphere`) (`GameplayStatics.GetPlayerCharacter` 0))
    (`Widget.SetVisibility` _ui_stats "Visible")
    (else
      (`Widget.SetVisibility` _ui_stats "Hidden")))
  (`self.UpdateWidget`)
  (set `/Game/Blueprints/UI/UI_Stats.NPC Name` (`KismetTextLibrary.Conv_StringToText` (`KismetSystemLibrary.GetDisplayName` self)) _ui_stats_2)
  (set `/Game/Blueprints/UI/UI_Stats.NPC Health` (`KismetTextLibrary.Conv_IntToText` (`self.Health`)) _ui_stats_2)
  (set `/Game/Blueprints/UI/UI_Stats.NPC isDead` (`KismetTextLibrary.Conv_BoolToText` (`self.isDead`)) _ui_stats_2)
  (set `/Game/Blueprints/UI/UI_Stats.Target Name` (`KismetTextLibrary.Conv_StringToText` (`KismetSystemLibrary.GetDisplayName` _currenttarget_2)) _ui_stats_2)
  (set `/Game/Blueprints/UI/UI_Stats.Target Distance` (`KismetTextLibrary.Conv_StringToText` (`KismetStringLibrary.Concat_StrStr` (`KismetStringLibrary.Conv_IntToString` (`KismetMathLibrary.FTrunc` (/ (`self.GetDistanceTo` _currenttarget_2) 100.0))) " m")) _ui_stats_2)
  (set `/Game/Blueprints/UI/UI_Stats.Target isDead` (`KismetTextLibrary.Conv_BoolToText` (`/Game/Blueprints/Characters/NPC_TeamA.isDead` _currenttarget_2)) _ui_stats_2)
  (set `/Game/Blueprints/UI/UI_Stats.Stat Color` (struct :`R` 0.109375 :`G` 0.040058 :`A` 0.755) _ui_stats_2)
  (set `/Game/Blueprints/UI/UI_Stats.NPC Color` (make `SlateColor` (struct :`R` 1.0 :`G` 0.564783 :`A` 1.0)) _ui_stats_2)
  (set `/Game/Blueprints/UI/UI_Stats.Target Color` (make `SlateColor` (struct :`G` 0.546875 :`B` 0.501967 :`A` 1.0)) _ui_stats_2)
  (set `/Game/Blueprints/UI/UI_Stats.NPC Janken` (`KismetTextLibrary.Conv_IntToText` (`self.Janken`)) _ui_stats_2)
  (if (<= (`self.Health`) 0)
    (set `self.isDead` true))
  (if (`self.isDead`)
    ;[0.4062 0 0] NPC is Dead
    (`/Engine/EditorBlueprintResources/StandardMacros.DoOnce` false
      (:`Completed`
        (`self.StopJumping`)
        (`PrimitiveComponent.SetSimulatePhysics` _mesh true)
        (`PrimitiveComponent.SetSimulatePhysics` (`self.CapsuleComponent`) true)
        (`PrimitiveComponent.SetCollisionEnabled` _mesh "QueryAndPhysics")
        (bind _outactors (`GameplayStatics.GetAllActorsOfClass` "NPC_TeamB_C"))
        (`KismetArrayLibrary.Array_RemoveItem` _outactors self)
        (`ActorComponent.K2_DestroyComponent` (`self.CapsuleComponent`))
        (`ActorComponent.K2_DestroyComponent` (`self.HitCapsule`))))
    (else
      (`self.Jump`)
      ;[1 0.9771 0] ENEMY DETECTION
      ;;[1 1 1 1 12] 1. On ajoute un délai aléatoire
      (`KismetSystemLibrary.Delay` (`KismetMathLibrary.RandomFloatInRange` 0.8 1.2))
      ;;[1 1 1 1 12] 2. On regarde si l'ennemi est en vie
      (if (`/Game/Blueprints/Characters/NPC_TeamA.isDead` (`self.CurrentTarget`))
        (`|ExecutionSequence`
          (:`then_0`
            (goto _label :!via `Reset`))
          (:`then_1`
            _)))
      ;;[1 1 1 1 12] 3. On regarde s'il y a des ennemis
      (bind _outactors_2 (`GameplayStatics.GetAllActorsOfClass` "/Game/Blueprints/Characters/NPC_TeamA.NPC_TeamA_C"))
      (bind _returnvalue_3 (`KismetArrayLibrary.Array_Length` _outactors_2))
      (if (> _returnvalue_3 0)
        (set `self.EnemyDeathCount` 0))
      ;;[1 1 1 1 12] 4. On cherche l'ennemi le plus proche
      (for _array_element _outactors_2
        (if (`/Game/Blueprints/Characters/NPC_TeamA.isDead` _array_element)
          (`/Engine/EditorBlueprintResources/StandardMacros.IncrementInt` (`self.EnemyDeathCount`)
            (:`  `
              (set `self.NearestEnemy` _enemyfindingrange)))
          (else
            (`|ExecutionSequence`
              (:`then_0`
                (`/Engine/EditorBlueprintResources/StandardMacros.DoOnce` false :!label _label
                  (:`Completed`
                    (set `self.NearestEnemy` _enemyfindingrange)
                    (bind _returnvalue_4 (`self.GetDistanceTo` _array_element))
                    (if (< _returnvalue_4 (`self.NearestEnemy`))
                      (set `self.NearestEnemy` _returnvalue_4)
                      (set `self.CurrentTarget` _array_element)))))
              (:`then_1`
                (if (< (`self.GetDistanceTo` _array_element) (`self.GetDistanceTo` (`self.CurrentTarget`)))
                  (set `self.CurrentTarget` _array_element)))))))
      ;;[1 1 1 1 12] 5. On regarde s'il reste des ennemis
      (if (< (`self.EnemyDeathCount`) _returnvalue_3)
        (set `self.EnemyDeathCount` 0)
        ;;[1 1 1 1 12] 6. On avance vers l'ennemi
        (`NavigationSystem.SimpleMoveToActor` (`self.GetController`) (`self.CurrentTarget`))
        ;[0.1159 0.06603 0.7604] Hit Event
        (if (`PrimitiveComponent.IsOverlappingComponent` (`self.HitCapsule`) (`Character.CapsuleComponent` (`self.CurrentTarget`)))
          (bind _output_get (set `self.Janken` (`KismetMathLibrary.RandomIntegerInRange` 0 100) :!label _label_2))
          (if (> _output_get _janken)
            (set `/Game/Blueprints/Characters/NPC_TeamA.Health` (- (`/Game/Blueprints/Characters/NPC_TeamA.Health` _currenttarget) (`KismetMathLibrary.RandomIntegerInRange` 10 15)) _currenttarget)
            (`self.LaunchCharacter` _currenttarget (`KismetMathLibrary.MakeVector` (.x (* (`self.GetActorForwardVector`) _returnvalue_2)) (.y (* (`self.GetActorForwardVector`) _returnvalue_2)) _returnvalue_2) false false)
            (`GameplayStatics.SpawnEmitterAtLocation` "/Game/StarterContent/Particles/P_Explosion.P_Explosion" (`self.K2_GetActorLocation` _currenttarget) (`KismetMathLibrary.RandomRotator` false) (`KismetMathLibrary.MakeVector` _returnvalue _returnvalue _returnvalue))
            (if (<= (`self.Health`) 0)
              (set `self.isDead` true))
            (elif (== _output_get _janken)
              (goto _label_2))))
        (else
          ;[0 0.3698 0.03469] VICTORY
          (`NavigationSystem.SimpleMoveToLocation` (`self.GetController`) (`self.SpawnLocation`))
          (set `self.CurrentTarget` null))))))

(event `self.CapsuleComponent.OnComponentHit`
  (params (HitComponent :type "PrimitiveComponent Object Reference") (OtherActor :type "Actor Object Reference") (OtherComp :type "PrimitiveComponent Object Reference") (NormalImpulse :type "Vector Structure") (Hit :type "HitResult Structure (by ref)"))
  (if (== (`GameplayStatics.GetObjectClass` OtherActor) "/Game/Blueprints/Characters/NPC_TeamA.NPC_TeamA_C")
    (bind _outactors (`GameplayStatics.GetAllActorsOfClass` "/Game/Blueprints/Characters/NPC_TeamA.NPC_TeamA_C"))
    (for _array_element _outactors
      (if (`KismetStringLibrary.EqualEqual_StrStr` (`KismetSystemLibrary.GetDisplayName` _array_element) (`KismetSystemLibrary.GetDisplayName` OtherActor))
        (set `self.CurrentTarget` _array_element)
        (set `self.NearestEnemy` (`self.EnemyFindingRange`))))))

(fn `CreateWidget`
  (bind _returnvalue (`|CreateWidget` "/Game/Blueprints/UI/UI_Stats.UI_Stats_C"))
  (bind _output_get (set `self.UI Stats` _returnvalue))
  (`UserWidget.AddToViewport` _output_get 0)
  (`Widget.SetVisibility` _output_get "Hidden")
  (`UserWidget.SetDesiredSizeInViewport` _output_get (100.0 65.0)))

(fn `UpdateWidget`
  (`UserWidget.SetPositionInViewport` (`self.UI Stats`) (- (`WidgetLayoutLibrary.ProjectWorldLocationToWidgetPosition` (`GameplayStatics.GetPlayerController` 0) (`SceneComponent.K2_GetComponentLocation` (`self.Mesh`))) (250.0 200.0)) false))

(fn `UserConstructionScript`)