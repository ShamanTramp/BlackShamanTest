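; TotemTeamA is a team A totem actor that shows an ice circle particle effect above itself and collapses when its health runs out.
; BeginPlay spawns the emitter, and every Tick copies Health to the player character's TotemHealth.
; At zero or less, Tick repeatedly enables physics on the five mesh parts, destroys the emitter and removes itself from a freshly fetched, otherwise unused array of TotemTeamA actors.
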(event `self.ReceiveBeginPlay`
  (bind _returnvalue (`GameplayStatics.SpawnEmitterAtLocation` "/Game/InfinityBladeEffects/Effects/FX_Mobile/ICE/combat/P_AOE_Ice_CircleAttack.P_AOE_Ice_CircleAttack" (`KismetMathLibrary.MakeVector` (.x (`self.K2_GetActorLocation`)) (.y (`self.K2_GetActorLocation`)) (+ (.z (`self.K2_GetActorLocation`)) 150.0)))))

(event `self.ReceiveTick`
  (params (DeltaSeconds :type "Float (single-precision)"))
  (bind _asfirst_person_character (cast `/Game/FirstPersonBP/Blueprints/FirstPersonCharacter` (`GameplayStatics.GetPlayerPawn` 0)))
  (set `/Game/FirstPersonBP/Blueprints/FirstPersonCharacter.TotemHealth` (`self.Health`) _asfirst_person_character)
  (if (<= (`self.Health`) 0)
    (`PrimitiveComponent.SetSimulatePhysics` (`self.Cube1`) true)
    (`PrimitiveComponent.SetSimulatePhysics` (`self.Cylinder`) true)
    (`PrimitiveComponent.SetSimulatePhysics` (`self.Cube`) true)
    (`PrimitiveComponent.SetSimulatePhysics` (`self.Sphere`) true)
    (`PrimitiveComponent.SetSimulatePhysics` (`self.Cone`) true)
    (`ActorComponent.K2_DestroyComponent` (stale `self.ReceiveBeginPlay` _returnvalue))
    (bind _outactors (`GameplayStatics.GetAllActorsOfClass` "TotemTeamA_C"))
    (`KismetArrayLibrary.Array_RemoveItem` _outactors self)))

(fn `UserConstructionScript`)